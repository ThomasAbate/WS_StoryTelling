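; BP_LastAutel is a chest VFX actor pairing a plane mesh with an FXChest Niagara effect, configured entirely in the construction script.
; ChestFXSize sets the plane's X and Y scale, flattened to zero on Z.
; A single Color variable tints the Niagara system and, multiplied for extra intensity, the plane's materials.
; The event graph holds only disabled placeholder events, so the Blueprint adds no runtime logic.
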(event EventBeginPlay)

(event Collision|EventActorBeginOverlap
  (params (OtherActor :type Actor%20Object%20Reference)))

(event EventTick
  (params (DeltaSeconds :type Float%20%28single-precision%29)))

(fn ConstructionScript
  (Transformation|SetWorldScale3D (Variables|Default|GetPlane) (* (Math|Conversions|ToVector(Vector2D) (Variables|Default|GetChestFXSize)) "0.005000,0.005000,0.005000"))
  (Niagara|SetNiagaraVariable(LinearColor) (Variables|Default|GetFX_Chest) "Color" (Variables|Default|GetColor))
  (Rendering|Material|SetVectorParameterValueonMaterials (Variables|Default|GetPlane) "Color" (Math|Conversions|ToVector(LinearColor) (* (Variables|Default|GetColor) "(R=5.000000,G=5.000000,B=5.000000,A=1.000000)"))))