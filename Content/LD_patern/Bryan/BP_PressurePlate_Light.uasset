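; BP_PressurePlate_Light is a pressure plate that reports its state changes to BP_Door_Light.
; Activation and Desactivation swap the plate mesh material, then call CheckSuccess on the first door found with GetActorOfClass.
; Desactivation also clears the door's IsWrongPlateActivated flag before that check.
; The event graph holds only disabled stubs, so nothing in this graph triggers either function.
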(event EventBeginPlay
  (|CallParentFunction) ; This node is disabled and will not be called.\nDrag off pins to build functionality.
)

(event Collision|EventActorBeginOverlap
  (params (OtherActor :type Actor%20Object%20Reference))
  (|CallParentFunction OtherActor) ; This node is disabled and will not be called.\nDrag off pins to build functionality.
)

(fn ConstructionScript
  (|CallParentFunction))

(fn Activation
  (Rendering|Material|SetMaterial (Variables|Default|GetPressurePlateMesh) 0 "/Engine/VREditor/UI/ArrowMaterial.ArrowMaterial")
  (bind _returnvalue (Actor|GetActorOfClass "/Game/LD_patern/Bryan/BP_Door_Light.BP_Door_Light_C"))
  (Default|CheckSuccess _returnvalue))

(fn Desactivation
  (Rendering|Material|SetMaterial (Variables|Default|GetPressurePlateMesh) 0 "/Engine/BasicShapes/BasicShapeMaterial.BasicShapeMaterial")
  (bind _returnvalue (Actor|GetActorOfClass "/Game/LD_patern/Bryan/BP_Door_Light.BP_Door_Light_C"))
  (Variables|/Game/LD_patern/Bryan/BP_Door_Light.BP_Door_Light_C|SetisWrongPlateActivated _returnvalue false)
  (Default|CheckSuccess _returnvalue))