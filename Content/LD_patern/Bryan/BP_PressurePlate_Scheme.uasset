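; Pressure plate Blueprint that gives visual feedback on activation, linking the plate to a target door and a set of other actors.
; Its Activation function loops over the NewVar array, swapping each element's Cube to a hue-shift material instance.
; Inside the same loop, it sets the plate mesh and the door target's bars to a shared basic material.
; The event graph holds only disabled default events, so nothing in this file calls Activation.
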(event EventBeginPlay
  (|CallParentFunction) ; This node is disabled and will not be called.\nDrag off pins to build functionality.
)

(event Collision|EventActorBeginOverlap
  (params (OtherActor :type Actor%20Object%20Reference))
  (|CallParentFunction OtherActor) ; This node is disabled and will not be called.\nDrag off pins to build functionality.
)

(event EventTick
  (params (DeltaSeconds :type Float%20%28single-precision%29))
  (|CallParentFunction DeltaSeconds) ; This node is disabled and will not be called.\nDrag off pins to build functionality.
)

(fn ConstructionScript
  (|CallParentFunction))

(fn Activation
  (for _array_element (Variables|Default|GetNewVar)
    (Rendering|Material|SetMaterial (Variables|/Game/LD_patern/Bryan/BP_ColorPlates.BP_ColorPlates_C|GetCube _array_element) 0 "/Engine/Functions/Engine_MaterialFunctions02/ExampleContent/HueShift_Inst.HueShift_Inst")
    (Rendering|Material|SetMaterial (Variables|Default|GetPressurePlateMesh) 0 "/Engine/MapTemplates/Materials/BasicAsset03.BasicAsset03")
    (Rendering|Material|SetMaterial (Variables|/Game/LD_patern/Bryan/BP_Barres_Porte.BP_Barres_Porte_C|GetBarres_Porte (Variables|Default|GetDoor%20Target)) 0 "/Engine/MapTemplates/Materials/BasicAsset03.BasicAsset03")))