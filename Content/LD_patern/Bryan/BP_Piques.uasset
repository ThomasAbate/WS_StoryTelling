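; BP_Piques is a level-design hazard prop, spikes by its French name, that rapidly bobs its Cube component up and down along relative Z.
; BeginPlay starts the motion, then the custom events Loop and Loop2 call each other after each latent MoveComponentTo, creating an endless oscillation without Tick.
; It contains no damage or overlap logic.
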(event Custom|Loop
  (Components|MoveComponentTo (Variables|Default|GetCube) (Math|Vector|MakeVector 0.0 0.0 -1e+01) "0, 0, 0" false false 0.1 false)
  (CallFunction|Loop2))

(event Custom|Loop2
  (Components|MoveComponentTo (Variables|Default|GetCube) (Math|Vector|MakeVector 0.0 0.0 1e+01) "0, 0, 0" false false 0.1 false)
  (CallFunction|Loop))

(event EventBeginPlay
  (Components|MoveComponentTo (Variables|Default|GetCube) (Math|Vector|MakeVector 0.0 0.0 1e+01) "0, 0, 0" false false 0.1 false)
  (CallFunction|Loop))

(event Collision|EventActorBeginOverlap
  (params (OtherActor :type Actor%20Object%20Reference)))

(event EventTick
  (params (DeltaSeconds :type Float%20%28single-precision%29)))

(fn ConstructionScript)