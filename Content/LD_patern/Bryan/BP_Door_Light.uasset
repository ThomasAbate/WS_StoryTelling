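; BP_Door_Light is a pressure plate puzzle door that opens when all its right plates are active and no wrong plate has been flagged.
; BeginPlay stores the right plate count, and CheckSuccess counts the active ones, printing a win message and calling DoorOpening on a match.
; The wrong plate scan runs after that test, so it only affects later checks, and this file never clears its flag.
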(event Custom|CheckSuccess
  (Variables|Default|SetcurrenttPressurePlateNumber 0)
  (Utilities|FlowControl|Sequence
    (:then_0
      (for _array_element (Variables|Default|GetRightPressurePlates)
        (if (Variables|/Game/Blueprints/BP_PressurePlate.BP_PressurePlate_C|GetisActivated _array_element)
          (Variables|Default|SetcurrenttPressurePlateNumber (+ (Variables|Default|GetcurrenttPressurePlateNumber) 1))
          (if (== (Variables|Default|GetRightPressurePlateNumber) (Variables|Default|GetcurrenttPressurePlateNumber))
            (if (not (Variables|Default|GetisWrongPlateActivated))
              (Development|PrintString "Win ! ")
              (CallFunction|DoorOpening))))))
    (:then_1
      (for _array_element_2 (Variables|Default|GetWrongPressurePlates)
        (if (Variables|/Game/Blueprints/BP_PressurePlate.BP_PressurePlate_C|GetisActivated _array_element_2)
          (Variables|Default|SetisWrongPlateActivated true))))))

(event EventBeginPlay
  (Variables|Default|SetRightPressurePlateNumber (Utilities|Array|Length (Variables|Default|GetRightPressurePlates))))

(event Collision|EventActorBeginOverlap
  (params (OtherActor :type Actor%20Object%20Reference))
  (|CallParentFunction OtherActor) ; This node is disabled and will not be called.\nDrag off pins to build functionality.
)

(event EventTick
  (params (DeltaSeconds :type Float%20%28single-precision%29))
  (|CallParentFunction DeltaSeconds) ; This node is disabled and will not be called.\nDrag off pins to build functionality.
)

(fn ConstructionScript
  (|CallParentFunction))