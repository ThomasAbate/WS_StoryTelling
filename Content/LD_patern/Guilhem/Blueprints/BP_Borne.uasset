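; BP_Borne is a rotating puzzle element that steps through positions and reports to a BP_BorneChecker.
; Activation and Desactivation are identical: each increments CurrentPosition, calls CheckSuccess on the checker found by class, then turns the Cube 90 degrees instantly.
; The position wraps to 0 on reaching 4, after the check has already run.
; An unconnected Timeline is left in the event graph.
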(event Custom|RotatingMovement
  (Transformation|AddLocalRotation (Variables|Default|GetCube) "0.000000,90.000000,0.000000" false false))

(event EventBeginPlay
  (|CallParentFunction) ; This node is disabled and will not be called.\nDrag off pins to build functionality.
)

(event Collision|EventActorBeginOverlap
  (params (OtherActor :type Actor%20Object%20Reference))
  (|CallParentFunction OtherActor) ; This node is disabled and will not be called.\nDrag off pins to build functionality.
)

(event EventTick
  (params (DeltaSeconds :type Float%20%28single-precision%29))
  (|CallParentFunction DeltaSeconds) ; This node is disabled and will not be called.\nDrag off pins to build functionality.
)

(fn ConstructionScript
  (|CallParentFunction))

(fn Activation
  (bind _output_get (Variables|Default|SetcurrentPosition (+ (Variables|Default|GetcurrentPosition) 1)))
  (bind _returnvalue (Actor|GetActorOfClass "/Game/LD_patern/Guilhem/Blueprints/BP_BorneChecker.BP_BorneChecker_C"))
  (Default|CheckSuccess _returnvalue)
  (CallFunction|RotatingMovement)
  (if (== _output_get 4)
    (Variables|Default|SetcurrentPosition 0)))

(fn Desactivation
  (bind _output_get (Variables|Default|SetcurrentPosition (+ (Variables|Default|GetcurrentPosition) 1)))
  (bind _returnvalue (Actor|GetActorOfClass "/Game/LD_patern/Guilhem/Blueprints/BP_BorneChecker.BP_BorneChecker_C"))
  (Default|CheckSuccess _returnvalue)
  (CallFunction|RotatingMovement)
  (if (== _output_get 4)
    (Variables|Default|SetcurrentPosition 0)))