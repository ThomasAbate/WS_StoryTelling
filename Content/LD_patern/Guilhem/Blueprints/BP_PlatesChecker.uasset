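; BP_PlatesChecker is a puzzle checker that opens a chest once every pressure plate pattern in its Patterns array is confirmed.
; At BeginPlay it stores the array length as the required count.
; CheckSuccess, which nothing in this file calls, recounts confirmed patterns from zero and calls ChestOpening when the count matches, printing debug strings along the way.
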(event EventBeginPlay
  (Variables|Default|SetRightPressurePlateNumber (Utilities|Array|Length (Variables|Default|GetPatterns))))

(fn ConstructionScript
  (|CallParentFunction))

(fn CheckSuccess
  (Variables|Default|SetcurrentCheckNumber 0)
  (for _array_element (Variables|Default|GetPatterns)
    (if (Variables|/Game/LD_patern/Guilhem/Blueprints/BP_PressurePlatePatternChecker.BP_PressurePlatePatternChecker_C|GetPatternIsConfirmed _array_element)
      (bind _output_get (Variables|Default|SetcurrentCheckNumber (+ (Variables|Default|GetcurrentCheckNumber) 1)))
      (Development|PrintString (Utilities|String|ToString(Integer) _output_get))
      (if (== _output_get (Variables|Default|GetRightPressurePlateNumber))
        (CallFunction|ChestOpening)
        (Development|PrintString "GG")))))