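; BP_BorneChecker is a puzzle controller that raises a pillar and chest when every linked borne is set to its correct position.
; BeginPlay stores the borne count, and CheckSuccess compares each borne's CurrentPosition to its RightPosition, printing debug messages for matches.
; When all match, ChestOpening plays the PillarAnim timeline, lerping the cylinder and chest upward.
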(event Custom|ChestOpening
  (bind _newtrack_0 (Timeline|PillarAnim Play)
    (:Update
      (Transformation|SetRelativeLocation (Variables|Default|GetCylinder) (Math|Vector|Lerp(Vector) "0, 0, 0" "0.000000,0.000000,360.000000" _newtrack_0) false false)
      (Transformation|SetRelativeLocation (Variables|/Script/Engine.Actor|GetRootComponent (Variables|Default|GetChest)) (Math|Vector|Lerp(Vector) "0.000000,0.000000,75.000000" "0.000000,0.000000,430.000000" _newtrack_0) false false))))

(event EventBeginPlay
  (Variables|Default|SetbornesNumber (Utilities|Array|Length (Variables|Default|GetBornes))))

(event Collision|EventActorBeginOverlap
  (params (OtherActor :type Actor%20Object%20Reference)))

(event EventTick
  (params (DeltaSeconds :type Float%20%28single-precision%29)))

(fn ConstructionScript)

(fn CheckSuccess
  (Variables|Default|SetcurrentCheckNumber 0)
  (for _array_element (Variables|Default|GetBornes)
    (if (== (Variables|/Game/LD_patern/Guilhem/Blueprints/BP_Borne.BP_Borne_C|GetcurrentPosition _array_element) (Variables|/Game/LD_patern/Guilhem/Blueprints/BP_Borne.BP_Borne_C|GetRightPosition _array_element))
      (bind _output_get (Variables|Default|SetcurrentCheckNumber (+ (Variables|Default|GetcurrentCheckNumber) 1)))
      (Development|PrintString (Utilities|String|ToString(Integer) _output_get))
      (Development|PrintString "Good Bornes")
      (if (== (Variables|Default|GetcurrentCheckNumber) (Variables|Default|GetbornesNumber))
        (Development|PrintString "Win !")
        (CallFunction|ChestOpening)))))