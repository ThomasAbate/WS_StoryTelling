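; Pressure plate puzzle checker that activates its bars when every right plate is active and no wrong plate is.
; On BeginPlay it registers itself with all right and wrong plates and stores the required count.
; CheckSuccess tallies active right plates and sets a wrong-plate flag that it never clears.
; On success it also marks the pattern confirmed and calls CheckSuccess on the level's BP_PlatesChecker, inside the per-bar loop.
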(event EventBeginPlay
  (for _array_element (Variables|Default|GetRightPressurePlate)
    (Variables|/Game/LD_patern/Bryan/BP_PressurePlate_Light.BP_PressurePlate_Light_C|SetPlates%20Checker _array_element self))
  (for _array_element_2 (Variables|Default|GetWrongPressurePlate)
    (Variables|/Game/LD_patern/Bryan/BP_PressurePlate_Light.BP_PressurePlate_Light_C|SetPlates%20Checker _array_element_2 self))
  (Variables|Default|SetRight%20Pressure%20Plate%20Number (Utilities|Array|Length (Variables|Default|GetRightPressurePlate))))

(fn ConstructionScript
  (|CallParentFunction))

(fn CheckSuccess
  (Variables|Default|SetCurrent%20Check%20Number 0)
  (for _array_element (Variables|Default|GetWrongPressurePlate)
    (if (Variables|/Game/Blueprints/BP_PressurePlate.BP_PressurePlate_C|GetisActivated _array_element)
      (Variables|Default|SetIs%20Wrong%20Plate%20Activated true)))
  (for _array_element_2 (Variables|Default|GetRightPressurePlate)
    (if (Variables|/Game/Blueprints/BP_PressurePlate.BP_PressurePlate_C|GetisActivated _array_element_2)
      (Variables|Default|SetCurrent%20Check%20Number (+ (Variables|Default|GetCurrent%20Check%20Number) 1))
      (if (== (Variables|Default|GetRight%20Pressure%20Plate%20Number) (Variables|Default|GetCurrent%20Check%20Number))
        (if (not (Variables|Default|GetIs%20Wrong%20Plate%20Activated))
          (for _array_element_3 (Variables|Default|GetBarsToActivate)
            (Default|Activation _array_element_3)
            (Variables|Default|SetPatternIsConfirmed true)
            (bind _returnvalue (Actor|GetActorOfClass "/Game/LD_patern/Guilhem/Blueprints/BP_PlatesChecker.BP_PlatesChecker_C"))
            (Default|CheckSuccess _returnvalue)))))))