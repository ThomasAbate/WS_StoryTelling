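; Tutorial pressure plate Blueprint that raises two referenced stair actors when activated.
; BeginPlay stores each stair's starting location.
; Activation calls StairUp, which plays a timeline that lerps both stairs straight up by a fixed offset from those stored positions, without sweeping.
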(event Custom|Stair%20Up
  (bind _first_stair_location (Variables|Default|GetFirst%20Stair%20Location))
  (bind _second_stair_location (Variables|Default|GetSecond%20Stair%20Location))
  (bind _alpha (Timeline|Stair%20Animation Play)
    (:Update
      (Transformation|SetActorLocation (Variables|Default|GetFirst%20Stair) (Math|Vector|Lerp(Vector) _first_stair_location (+ _first_stair_location "0.000000,0.000000,500.000000") _alpha) false false)
      (Transformation|SetActorLocation (Variables|Default|GetSecond%20Stair) (Math|Vector|Lerp(Vector) _second_stair_location (+ _second_stair_location "0.000000,0.000000,500.000000") _alpha) false false))))

(event EventBeginPlay
  (Variables|Default|SetFirst%20Stair%20Location (Transformation|GetActorLocation (Variables|Default|GetFirst%20Stair)))
  (Variables|Default|SetSecond%20Stair%20Location (Transformation|GetActorLocation (Variables|Default|GetSecond%20Stair))))

(fn ConstructionScript
  (|CallParentFunction))

(fn Activation
  (CallFunction|StairUp))