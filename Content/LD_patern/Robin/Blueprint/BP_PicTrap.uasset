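; Spike trap Blueprint that slides its spike component out in two stages: a warning move, then an attack.
; Activation runs ActivationAnim, which moves the spike to a prevention distance, waits, then moves it to the attack distance at configurable speed.
; A sound call at the world origin follows the attack move.
; After a fixed delay, the spike retracts and IsActivated on ActivateTriggerBox is cleared.
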(event Custom|ActivationAnim
  (bind _trapspeed (Variables|Default|GetTrapSpeed))
  (bind _bp_pique (Variables|Default|GetBP_Pique))
  (Components|MoveComponentTo _bp_pique (Math|Vector|MakeVector (Variables|Default|GetPreventionDistance) 0.0 0.0) "0.000000,-90.000000,0.000000" false false _trapspeed false)
  (Utilities|FlowControl|Delay (Variables|Default|GetPreventionDelay))
  (Components|MoveComponentTo _bp_pique (Math|Vector|MakeVector (Variables|Default|GetAttackDistance) 0.0 0.0) "0.000000,-90.000000,0.000000" false false _trapspeed false)
  (Audio|PlaySoundatLocation "/Game/Sound/Spikes.Spikes" "0, 0, 0" "0, 0, 0" 1.0 1.0 0.0 0 0 0 0)
  (Utilities|FlowControl|Delay 2.0)
  (Components|MoveComponentTo _bp_pique (Math|Vector|MakeVector 0.0 0.0 0.0) "0.000000,-90.000000,0.000000" false false 0.2 false)
  (Variables|/Game/Blueprints/BP_Parent/BP_TriggerBox.BP_TriggerBox_C|SetisActivated (Variables|Default|GetActivateTriggerBox) false))

(fn ConstructionScript
  (|CallParentFunction))

(fn Activation
  (CallFunction|ActivationAnim))