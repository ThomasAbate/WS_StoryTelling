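; Moving platform Blueprint that carries its static mesh between its initial relative transform and a Destination offset, starting at BeginPlay.
; A timeline, with play rate set from the travel time, lerps location and rotation together.
; Rotation lerp inputs run opposite to location, blending from the offset rotation toward the initial one.
; When the timeline finishes, a pause feeds a FlipFlop that alternates play and reverse calls.
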(event Custom|Start%20Movement
  (bind _initrot (Variables|Default|GetInitRot))
  (bind _destination (Variables|Default|GetDestination))
  (bind _initpos (Variables|Default|GetInitPos))
  (bind _alpha (Timeline|Animator Play)
    (:Update
      ;[1 1 1] Move Platform
      (Variables|Default|SetLerpAlpha _alpha)
      (Transformation|SetRelativeLocationAndRotation (Variables|Default|GetStaticMesh) (Math|Vector|Lerp(Vector) _initpos (+ _initpos (.location _destination)) (Variables|Default|GetLerpAlpha)) (Math|Rotator|Lerp(Rotator) (Math|Rotator|CombineRotators (.rotation _destination) _initrot) _initrot (Variables|Default|GetLerpAlpha)) false false))
    (:Finished
      (Utilities|FlowControl|Delay (Variables|Default|GetPause%20Time))
      (Utilities|FlowControl|FlipFlop
        (:A
          (CallFunction|StartMovement))
        (:B
          (CallFunction|ReverseMovement))))))

(event Custom|Reverse%20Movement
  (bind _initrot (Variables|Default|GetInitRot))
  (bind _destination (Variables|Default|GetDestination))
  (bind _initpos (Variables|Default|GetInitPos))
  (bind _alpha (Timeline|Animator Reverse)
    (:Update
      ;[1 1 1] Move Platform
      (Variables|Default|SetLerpAlpha _alpha)
      (Transformation|SetRelativeLocationAndRotation (Variables|Default|GetStaticMesh) (Math|Vector|Lerp(Vector) _initpos (+ _initpos (.location _destination)) (Variables|Default|GetLerpAlpha)) (Math|Rotator|Lerp(Rotator) (Math|Rotator|CombineRotators (.rotation _destination) _initrot) _initrot (Variables|Default|GetLerpAlpha)) false false))
    (:Finished
      (Utilities|FlowControl|Delay (Variables|Default|GetPause%20Time))
      (Utilities|FlowControl|FlipFlop
        (:A
          (CallFunction|StartMovement))
        (:B
          (CallFunction|ReverseMovement))))))

(event EventBeginPlay
  (bind _staticmesh (Variables|Default|GetStaticMesh))
  (bind _returnvalue (Transformation|GetRelativeTransform _staticmesh))
  (Variables|Default|SetInitPos (.location _returnvalue))
  (Variables|Default|SetInitRot (.rotation _returnvalue))
  (Components|Timeline|SetPlayRate (Variables|Default|GetAnimator) (/ 1.0 (Variables|Default|GetTravelTimeInSecond)))
  (CallFunction|StartMovement))

(fn ConstructionScript)