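; BP_BorneChecker_Fifth is a puzzle checker that opens a Door when enough Bornes are in their correct positions.
; CheckSuccess resets a counter, loops over the Bornes array and counts each one whose CurrentPosition equals its RightPosition.
; When the count reaches BornesNumber it calls Activation on the Door, printing progress and win messages as debug strings.
; The event graph holds only disabled default events, and nothing in this Blueprint calls CheckSuccess.
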(event EventBeginPlay
  (|CallParentFunction) ; This node is disabled and will not be called.\nDrag off pins to build functionality.
)

(event Collision|EventActorBeginOverlap
  (params (OtherActor :type Actor%20Object%20Reference))
  (|CallParentFunction OtherActor) ; This node is disabled and will not be called.\nDrag off pins to build functionality.
)

(event EventTick
  (params (DeltaSeconds :type Float%20%28single-precision%29))
  (|CallParentFunction DeltaSeconds) ; This node is disabled and will not be called.\nDrag off pins to build functionality.
)

(fn ConstructionScript
  (|CallParentFunction))

(fn CheckSuccess
  (Variables|Default|SetcurrentCheckNumber 0)
  (for _array_element (Variables|Default|GetBornes)
    (if (== (Variables|/Game/LD_patern/Guilhem/Blueprints/BP_Borne.BP_Borne_C|GetcurrentPosition _array_element) (Variables|/Game/LD_patern/Guilhem/Blueprints/BP_Borne.BP_Borne_C|GetRightPosition _array_element))
      (bind _output_get (Variables|Default|SetcurrentCheckNumber (+ (Variables|Default|GetcurrentCheckNumber) 1)))
      (Development|PrintString (Utilities|String|ToString(Integer) _output_get))
      (Development|PrintString "Good Bornes")
      (if (== (Variables|Default|GetcurrentCheckNumber) (Variables|Default|GetbornesNumber))
        (Development|PrintString "Win !")
        (Default|Activation (Variables|Default|GetDoor))))))