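; Trapdoor trap that opens two panels when activated.
; The Activation function calls the ActivationAnim event, which uses MoveComponentTo to rotate the Cube and Cube1 components a quarter turn in opposite directions.
; Desactivation is empty, so nothing here closes the trapdoor again.
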(event Custom|ActivationAnim
  (Utilities|FlowControl|Sequence
    (:then_0
      (Components|MoveComponentTo (Variables|Default|GetCube) "0, 0, 0" "-90.000000,0.000000,0.000000" false false 0.2 false))
    (:then_1
      (Components|MoveComponentTo (Variables|Default|GetCube1) "0, 0, 0" "90.000000,0.000000,0.000000" false false 0.2 false))))

(event EventBeginPlay
  (|CallParentFunction) ; This node is disabled and will not be called.\nDrag off pins to build functionality.
)

(event Collision|EventActorBeginOverlap
  (params (OtherActor :type Actor%20Object%20Reference))
  (|CallParentFunction OtherActor) ; This node is disabled and will not be called.\nDrag off pins to build functionality.
)

(event EventTick
  (params (DeltaSeconds :type Float%20%28single-precision%29))
  (|CallParentFunction DeltaSeconds) ; This node is disabled and will not be called.\nDrag off pins to build functionality.
)

(fn ConstructionScript
  (|CallParentFunction))

(fn Activation
  (CallFunction|ActivationAnim))

(fn Desactivation)