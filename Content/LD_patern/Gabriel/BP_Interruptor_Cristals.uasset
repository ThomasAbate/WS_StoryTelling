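; BP_Interruptor_Cristals is a level-design switch actor, named for crystals, that slides a grid mesh to a lowered position when activated.
; Its Activation function calls the Minus event, which uses MoveComponentTo to move the grid's GridPolySurface6 component to a negative relative Z over a short time.
; No logic here raises the grid again or detects the trigger, and BeginPlay, overlap and Tick are disabled stubs.
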(event Custom|Minus
  (Components|MoveComponentTo (Variables|/Game/MESHES/ENVIRO/Grid_Actor.Grid_Actor_C|GetGrid_polySurface6 (Variables|Default|GetGrid)) (Math|Vector|MakeVector 0.0 0.0 -1e+02) "0, 0, 0" false false 0.4 false))

(event EventBeginPlay
  (|CallParentFunction) ; This node is disabled and will not be called.\nDrag off pins to build functionality.
)

(event Collision|EventActorBeginOverlap
  (params (OtherActor :type Actor%20Object%20Reference))
  (|CallParentFunction OtherActor) ; This node is disabled and will not be called.\nDrag off pins to build functionality.
)

(event EventTick
  (params (DeltaSeconds :type Float%20%28single-precision%29))
  (|CallParentFunction DeltaSeconds) ; This node is disabled and will not be called.\nDrag off pins to build functionality.
)

(fn ConstructionScript
  (|CallParentFunction))

(fn Activation
  (CallFunction|Minus))