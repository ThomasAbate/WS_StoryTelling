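; BP_EnterRoom plays a one-time camera cutscene, named as a room entrance, when its Activation function is called.
; EnterCamera disables player input, blends the view to CameraTarget, then creates and plays a Level Sequence.
; A fixed delay, rather than a sequence-finished event, times the blend back to the player character and the return of input.
; A DoOnce prevents the cutscene from replaying on later activations.
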(event Custom|EnterCamera
  (Utilities|FlowControl|DoOnce false
    (:Completed
      (Input|DisableInput (Game|GetPlayerCharacter 0) (Game|GetPlayerController 0))
      (Game|Player|SetViewTargetwithBlend (Game|GetPlayerController 0) (Variables|Default|GetCameraTarget) 1.0 "VTBlend_EaseInOut" 1e+01 false)
      (Utilities|FlowControl|Delay 1.0)
      (bind _returnvalue (Sequencer|Player|CreateLevelSequencePlayer (Variables|Default|GetLevel%20Sequence)))
      (Sequencer|Player|Play _returnvalue :!class /Script/MovieScene.MovieSceneSequencePlayer)
      (Utilities|FlowControl|Delay 6.7)
      (Game|Player|SetViewTargetwithBlend (Game|GetPlayerController 0) (Game|GetPlayerCharacter 0) 1.0 "VTBlend_EaseInOut" 1e+01 false)
      (Input|EnableInput (Game|GetPlayerCharacter 0) (Game|GetPlayerController 0)))))

(fn ConstructionScript
  (|CallParentFunction))

(fn Activation
  (CallFunction|EnterCamera))