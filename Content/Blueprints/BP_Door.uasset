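; Two-panel door that slides open and closed through Activation and Desactivation, with a short camera sequence on opening.
; Activation starts a camera shake and DoorOpening, which disables player input, blends the view to CameraTarget, plays a sound and moves both panels.
; Each finished move turns the player toward the door, triggers rumble, restores view and input, and switches to the end sound.
; DoorClosing only moves the panels to positions cached at BeginPlay, offsetting the right one.
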(event Custom|DoorClosing
  (Utilities|FlowControl|Sequence
    (:then_0
      (Components|MoveComponentTo (Variables|Default|GetDoorLeft) (Variables|Default|GetDoorLeftPos) "0.000000,90.000000,0.000000" false false (Variables|Default|GetClosingTime) false))
    (:then_1
      (Components|MoveComponentTo (Variables|Default|GetDoorRight) (- (Variables|Default|GetDoorRightPos) "250.000000,0.000000,0.000000") "0.000000,90.000000,0.000000" false false (Variables|Default|GetClosingTime) false))))

(event Custom|DoorOpening
  (bind _audiocomponent (Variables|Default|GetAudioComponent))
  (Input|DisableInput (Game|GetPlayerCharacter 0) (Game|GetPlayerController 0))
  (Game|Player|SetViewTargetwithBlend (Game|GetPlayerController 0) (Variables|Default|GetCamera%20Target) 0.2 "VTBlend_PreBlended" 0.2 false)
  (Utilities|FlowControl|Sequence
    (:then_0
      (Components|MoveComponentTo (Variables|Default|GetDoorLeft) (.location (Variables|Default|GetDestinationLeft)) "0.000000,90.000000,0.000000" false false (Variables|Default|GetClosingTime) false)
      (Utilities|FlowControl|Sequence :!label _label
        (:then_0
          (CallFunction|LookatDoor)
          (Game|Feedback|PlayDynamicForceFeedback (Game|GetPlayerController 0) 0.1 0.2 true true true true)
          (Game|Player|SetViewTargetwithBlend (Game|GetPlayerController 0) (Game|GetPlayerCharacter 0) 1.0 "VTBlend_EaseInOut" 1e+01 false)
          (Input|EnableInput (Game|GetPlayerCharacter 0) (Game|GetPlayerController 0)))
        (:then_1
          (Audio|PlaySoundatLocation "/Game/Sound/DoorOpen_END.DoorOpen_END" "0, 0, 0" "0, 0, 0" 1.0 1.0 0.0 0 0 0 0)
          (Audio|Components|Audio|Stop (Variables|Default|GetAudioComponent)))))
    (:then_1
      (Components|MoveComponentTo (Variables|Default|GetDoorRight) (- (.location (Variables|Default|GetDestinationRight)) "250.000000,0.000000,0.000000") "0.000000,90.000000,0.000000" false false (Variables|Default|GetClosingTime) false)
      (goto _label))
    (:then_2
      (Audio|Components|Audio|SetSound _audiocomponent (Variables|Default|GetSound))
      (Audio|Components|Audio|Play _audiocomponent 0.0)
      (Transformation|SetWorldLocation _audiocomponent "0, 0, 0" false false))))

(event EventBeginPlay
  (|CallParentFunction)
  (Variables|Default|SetDoorRightPos (Transformation|GetWorldLocation (Variables|Default|GetDoorRight)))
  (Variables|Default|SetDoorLeftPos (Transformation|GetWorldLocation (Variables|Default|GetDoorLeft))))

(fn ConstructionScript
  (|CallParentFunction))

(fn Activation
  (CallFunction|DoorOpening)
  (Class|LegacyCameraShake|StartLegacyCameraShake (Game|GetPlayerCameraManager 0) (Variables|Default|GetShake%20Class) 1.0 "CameraLocal" "0, 0, 0"))

(fn Desactivation
  (CallFunction|DoorClosing))

(fn LookatDoor
  (bind _returnvalue (Game|GetPlayerCharacter 0))
  (Pawn|SetControlRotation (Pawn|GetController _returnvalue) (Math|Rotator|FindLookatRotation (Transformation|GetActorLocation _returnvalue) (Transformation|GetActorLocation))))