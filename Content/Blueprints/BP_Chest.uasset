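; BP_Chest is an activatable chest that awards an idol fragment.
; Activation starts an animation that plays a sound at world origin, rotates the lid open and hides the BPChest component after a delay.
; It also calls the game mode's idol WidgetUpdate, then increments the fragment count.
; After calling the parent Activation, it asks the BP_FinalAutel actor, if found, to check validity.
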(event Custom|ActivationAnim
  (Audio|PlaySoundatLocation "/Game/Sound/Chest_Open.Chest_Open" "0, 0, 0" "0, 0, 0" 1.0 1.0 0.0 0 0 0 0)
  (Components|MoveComponentTo (Variables|Default|Getcoffre_1_pasted__haut) "0, 0, 0" "35.000000,0.000000,0.000000" false false 0.5 false)
  (Utilities|FlowControl|Delay 1.0)
  (Rendering|SetVisibility (Variables|Default|GetBP_Chest) false false))

(event EventBeginPlay
  (|CallParentFunction))

(event Collision|EventActorBeginOverlap
  (params (OtherActor :type Actor%20Object%20Reference))
  (|CallParentFunction OtherActor) ; This node is disabled and will not be called.\nDrag off pins to build functionality.
)

(event EventTick
  (params (DeltaSeconds :type Float%20%28single-precision%29))
  (|CallParentFunction DeltaSeconds) ; This node is disabled and will not be called.\nDrag off pins to build functionality.
)

(fn ConstructionScript
  (|CallParentFunction))

(fn Activation
  (bind _returnvalue (Game|GetGameMode))
  (bind _asbp_third_person_game_mode (Utilities|Casting|CastToBP_ThirdPersonGameMode _returnvalue))
  (CallFunction|ActivationAnim)
  (Default|WidgetUpdate (Variables|/Game/Blueprints/ThirdPerson/Blueprints/BP_ThirdPersonGameMode.BP_ThirdPersonGameMode_C|GetWidgetIdole _asbp_third_person_game_mode))
  (Variables|/Game/Blueprints/ThirdPerson/Blueprints/BP_ThirdPersonGameMode.BP_ThirdPersonGameMode_C|SetIdoleFragmentCurrent _asbp_third_person_game_mode (+ (Variables|/Game/Blueprints/ThirdPerson/Blueprints/BP_ThirdPersonGameMode.BP_ThirdPersonGameMode_C|GetIdoleFragmentCurrent _asbp_third_person_game_mode) 1))
  (|CallParentFunction)
  (bind _returnvalue_2 (Actor|GetActorOfClass "/Game/Blueprints/BP_FinalAutel.BP_FinalAutel_C"))
  (Utilities|IsValid _returnvalue_2
    (:Is%20Valid
      (Default|CheckValidity _returnvalue_2))))