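; BP_Final_Rock_Systeme is a level system actor that triggers the final rock sequence through its Activation function.
; Activation spawns a BP_Final_Rock at the actor's root transform, passing it the FinalPoint variable.
; It also spawns a BP_Camera_Final_Rock at TargetPointCam and smoothly blends the player's view to that camera.
; The event graph is empty, so nothing runs until Activation is called externally.
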(event EventBeginPlay)

(event Collision|EventActorBeginOverlap
  (params (OtherActor :type Actor%20Object%20Reference))
  (|CallParentFunction OtherActor) ; This node is disabled and will not be called.\nDrag off pins to build functionality.
)

(event EventTick
  (params (DeltaSeconds :type Float%20%28single-precision%29))
  (|CallParentFunction DeltaSeconds) ; This node is disabled and will not be called.\nDrag off pins to build functionality.
)

(fn ConstructionScript
  (|CallParentFunction))

(fn Activation
  (Game|SpawnActorfromClass "/Game/Blueprints/GPE/Lethal/BP_Final_Rock.BP_Final_Rock_C" (Transformation|GetWorldTransform (Variables|Default|GetDefaultSceneRoot)) "Undefined" "MultiplyWithRoot" 0 (Variables|Default|GetFinal%20Point) 0)
  (bind _returnvalue (Game|SpawnActorfromClass "/Game/Blueprints/Level_Systems/System_L_Rock/BP_Camera_Final_Rock.BP_Camera_Final_Rock_C" (Transformation|GetActorTransform (Variables|Default|GetTarget%20Point%20Cam)) "Undefined" "MultiplyWithRoot" 0 0))
  (Game|Player|SetViewTargetwithBlend (Game|GetPlayerController 0) _returnvalue 1.5 "VTBlend_EaseInOut" 2.0 false))