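; Tutorial trigger volume that shows a widget on screen while the player's pawn is inside it.
; On begin overlap, it creates an instance of its Widget class for player 0, stores it in CurrentWidget and adds it to the viewport.
; On end overlap, it removes that widget from its parent and prints a "Hello" debug string.
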(event OnComponentBeginOverlap(Trigger)
  (params (OverlappedComponent :type Primitive%20Component%20Object%20Reference) (OtherActor :type Actor%20Object%20Reference) (OtherComp :type Primitive%20Component%20Object%20Reference) (OtherBodyIndex :type Integer) (bFromSweep :type Boolean) (SweepResult :type Hit%20Result%20Structure%20%28by%20ref%29))
  (if (== OtherActor (Game|Player|GetPlayerPawn 0))
    (CallFunction|AddWidget)))

(event OnComponentEndOverlap(Trigger)
  (params (OverlappedComponent :type Primitive%20Component%20Object%20Reference) (OtherActor :type Actor%20Object%20Reference) (OtherComp :type Primitive%20Component%20Object%20Reference) (OtherBodyIndex :type Integer))
  (if (== OtherActor (Game|Player|GetPlayerPawn 0))
    (CallFunction|DeletWidget)))

(event Custom|Add%20Widget
  (bind _returnvalue (UserInterface|CreateWidget (Variables|Default|GetWidget) (Game|GetPlayerController 0)))
  (bind _output_get (Variables|Default|SetCurrent%20Widget _returnvalue))
  (UserInterface|Viewport|AddtoViewport _output_get 0))

(event Custom|Delet%20Widget
  (Widget|RemovefromParent (Variables|Default|GetCurrent%20Widget))
  (Development|PrintString "Hello"))

(fn ConstructionScript)