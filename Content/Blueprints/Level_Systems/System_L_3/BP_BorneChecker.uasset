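; BP_BorneChecker is a puzzle manager that reveals a chest once every linked borne is in its correct position.
; CheckSuccess counts bornes whose current position matches the right one; a full match plays a validation sound, fires ChestOpening and activates linked bars.
; ChestOpening slides two traps open, then moves the altar cylinder and chest to the altar destination with audio cues.
; It also flags borne interactions as interacted and interact-once.
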(event Custom|ChestOpening
  (bind _destinationaltar (Variables|Default|GetDestinationAltar))
  (bind _openingtime (Variables|Default|GetOpeningTime))
  (bind _altartime (Variables|Default|GetAltarTime))
  (bind _audio (Variables|Default|GetAudio))
  (Utilities|FlowControl|Sequence
    (:then_0
      (Components|MoveComponentTo (Variables|Default|GetLeftTrap) (.location (Variables|Default|GetDestinationLeft)) "0, 0, 0" false false _openingtime false)
      (Audio|Components|Audio|Play (Variables|Default|GetAudio) 0.0 :!label _label)
      (Utilities|FlowControl|Sequence
        (:then_0
          (Components|MoveComponentTo (Variables|Default|GetCylinder) (+ (.location _destinationaltar) "-75.000000,75.000000,0.000000") "0, 0, 0" false false _altartime false))
        (:then_1
          (Components|MoveComponentTo (Variables|/Script/Engine.Actor|GetRootComponent (Variables|Default|GetChest)) (+ (.location _destinationaltar) "0.000000,0.000000,185.000000") "0, 0, 0" false false _altartime false)))
      (Audio|Components|Audio|SetSound _audio "/Game/Sound/SFX/Bornes/Borne_Checker_END.Borne_Checker_END")
      (Audio|Components|Audio|Play _audio 0.0))
    (:then_1
      (Components|MoveComponentTo (Variables|Default|GetRightTrap) (.location (Variables|Default|GetDestinationRight)) "0, 0, 0" false false _openingtime false)
      (goto _label))
    (:then_2
      (for _array_element (Variables|Default|GetBornesInteraction)
        (Variables|/Game/Blueprints/BP_Parent/BP_SystemInteractable.BP_SystemInteractable_C|SetisInteracted _array_element true)
        (Variables|/Game/Blueprints/BP_Parent/BP_SystemInteractable.BP_SystemInteractable_C|SetInteractableOnce _array_element true)))))

(event EventBeginPlay
  (Variables|Default|SetbornesNumber (Utilities|Array|Length (Variables|Default|GetBornes))))

(fn ConstructionScript)

(fn CheckSuccess
  (Variables|Default|SetcurrentCheckNumber 0)
  (for _array_element (Variables|Default|GetBornes)
    (if (== (Variables|/Game/Blueprints/GPE/BP_Borne.BP_Borne_C|GetcurrentPosition _array_element) (Variables|/Game/Blueprints/GPE/BP_Borne.BP_Borne_C|GetRightPosition _array_element))
      (Variables|Default|SetcurrentCheckNumber (+ (Variables|Default|GetcurrentCheckNumber) 1))
      (if (== (Variables|Default|GetcurrentCheckNumber) (Variables|Default|GetbornesNumber))
        (CallFunction|ChestOpening)
        (Audio|PlaySound2D "/Game/Sound/SFX/Validation.Validation" 1.0 1.0 0.0 0 0)
        (for _array_element_2 (Variables|Default|GetBarsToActivate)
          (Default|Activation _array_element_2))))))