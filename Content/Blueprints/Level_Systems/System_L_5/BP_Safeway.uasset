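; BP_Safeway is a level-system actor with one static mesh that moves or disappears when its Safeway event is called.
; With MoveY set, the mesh moves to TargetRelativeLocationY, taking the relative target's X and Z from its current world location.
; Otherwise, the mesh is hidden and its collision disabled.
; BeginPlay applies the Material variable to the mesh.
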(event Custom|Safeway
  (bind _staticmesh (Variables|Default|GetStaticMesh))
  (bind _returnvalue (Transformation|GetWorldLocation _staticmesh))
  (if (Variables|Default|GetMove_Y)
    (Components|MoveComponentTo _staticmesh (Math|Vector|MakeVector (.x _returnvalue) (Variables|Default|GetTarget%20Relative%20Location%20Y) (.z _returnvalue)) "0, 0, 0" false false 0.2 false)
    (else
      (Rendering|SetVisibility (Variables|Default|GetStaticMesh) false false)
      (Collision|SetCollisionEnabled (Variables|Default|GetStaticMesh) "NoCollision"))))

(event EventBeginPlay
  (Rendering|Material|SetMaterial (Variables|Default|GetStaticMesh) 0 (Variables|Default|GetMaterial)))

(fn ConstructionScript)