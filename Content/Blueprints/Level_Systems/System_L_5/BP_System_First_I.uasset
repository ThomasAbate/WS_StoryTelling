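; BP_System_First_I is a level-system actor that plays a scripted camera cutscene opening a level 5 door.
; Activation calls Movement, a Delay-timed sequence that disables player input and blends views from CameraTarget to CameraDoor and back to the player before restoring input.
; Along the way it turns the player toward TargetToLook, replaces the Crystal with FX and sound, lowers a Grid surface and triggers Door.DoorLVL5.
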(event Custom|Movement
  (bind _crystal (Variables|Default|GetCrystal))
  (Input|DisableInput (Game|GetPlayerCharacter 0) (Game|GetPlayerController 0))
  (Game|Player|SetViewTargetwithBlend (Game|GetPlayerController 0) (Variables|Default|GetCamera%20Target) 0.2 "VTBlend_PreBlended" 0.2 false)
  (Utilities|FlowControl|Delay 0.9)
  (CallFunction|SetPlayerCameraDirection)
  (Rendering|SetActorHiddenInGame _crystal true)
  (Game|SpawnActorfromClass "/Game/GA/VFX/BP_Crystal_FX.BP_Crystal_FX_C" (Transformation|GetActorTransform _crystal) "Undefined" "MultiplyWithRoot" 0 0)
  (Audio|PlaySoundatLocation "/Game/Sound/Rupee_SFX.Rupee_SFX" "0, 0, 0" "0, 0, 0" 1.0 1.0 0.0 0 0 0 0)
  (Utilities|FlowControl|Delay 1.5)
  (Components|MoveComponentTo (Variables|/Game/GA/MESHES/ENVIRO/Grid_Actor.Grid_Actor_C|GetGrid_polySurface6 (Variables|Default|GetGrid)) (Math|Vector|MakeVector 0.0 0.0 -1e+03) "0, 0, 0" false false 1.3 false)
  (Utilities|FlowControl|Delay 1.0)
  (Game|Player|SetViewTargetwithBlend (Game|GetPlayerController 0) (Variables|Default|GetCameraDoor) 1.0 "VTBlend_EaseInOut" 1e+01 false)
  (Utilities|FlowControl|Delay 0.9)
  (Default|DoorLVL5 (Variables|Default|GetDoor))
  (Utilities|FlowControl|Delay 1.0)
  (Game|Player|SetViewTargetwithBlend (Game|GetPlayerController 0) (Game|GetPlayerCharacter 0) 1.0 "VTBlend_EaseInOut" 1e+01 false)
  (Input|EnableInput (Game|GetPlayerCharacter 0) (Game|GetPlayerController 0)))

(event EventBeginPlay
  (|CallParentFunction) ; This node is disabled and will not be called.\nDrag off pins to build functionality.
)

(event Collision|EventActorBeginOverlap
  (params (OtherActor :type Actor%20Object%20Reference))
  (|CallParentFunction OtherActor) ; This node is disabled and will not be called.\nDrag off pins to build functionality.
)

(event EventTick
  (params (DeltaSeconds :type Float%20%28single-precision%29))
  (|CallParentFunction DeltaSeconds) ; This node is disabled and will not be called.\nDrag off pins to build functionality.
)

(fn ConstructionScript
  (|CallParentFunction))

(fn Activation
  (CallFunction|Movement))

(fn SetPlayerCameraDirection
  (bind _returnvalue (Game|GetPlayerCharacter 0))
  (Pawn|SetControlRotation (Pawn|GetController _returnvalue) (Math|Rotator|FindLookatRotation (Transformation|GetActorLocation _returnvalue) (Transformation|GetActorLocation (Variables|Default|GetTarget%20To%20Look)))))