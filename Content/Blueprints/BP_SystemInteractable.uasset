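; BP_SystemInteractable is an interactable actor that lets the player trigger a list of linked systems.
; Entering InteractableRadius flags the player character as able to interact, registers this actor as its current system and shows a tutorial prompt widget, unless it is single-use and already used.
; Leaving the radius clears that state and removes the prompt.
; Activation forwards the call to each valid entry in SystemsToActivate.
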(event OnComponentBeginOverlap(InteractableRadius)
  (params (OverlappedComponent :type Primitive%20Component%20Object%20Reference) (OtherActor :type Actor%20Object%20Reference) (OtherComp :type Primitive%20Component%20Object%20Reference) (OtherBodyIndex :type Integer) (bFromSweep :type Boolean) (SweepResult :type Hit%20Result%20Structure%20%28by%20ref%29))
  (bind _returnvalue (Game|GetPlayerCharacter 0))
  (bind _asbp_third_person_character (Utilities|Casting|CastToBP_ThirdPersonCharacter _returnvalue))
  (if (not (and (Variables|Default|GetInteractableOnce) (Variables|Default|GetisInteracted)))
    (if (== OtherActor _returnvalue)
      (Variables|/Game/ThirdPerson/Blueprints/BP_ThirdPersonCharacter.BP_ThirdPersonCharacter_C|SetIsCanInteract? _asbp_third_person_character true)
      (Variables|/Game/ThirdPerson/Blueprints/BP_ThirdPersonCharacter.BP_ThirdPersonCharacter_C|SetCurrentInteractSystem _asbp_third_person_character self)
      (bind _returnvalue_2 (UserInterface|CreateWidget "/Game/LD_patern/Thomas/Widget/WBP_Tuto_Interact.WBP_Tuto_Interact_C" (Game|GetPlayerController 0)))
      (bind _output_get (Variables|Default|SetInteractWidget _returnvalue_2))
      (UserInterface|Viewport|AddtoViewport _output_get 0))))

(event OnComponentEndOverlap(InteractableRadius)
  (params (OverlappedComponent :type Primitive%20Component%20Object%20Reference) (OtherActor :type Actor%20Object%20Reference) (OtherComp :type Primitive%20Component%20Object%20Reference) (OtherBodyIndex :type Integer))
  (bind _returnvalue (Game|GetPlayerCharacter 0))
  (bind _asbp_third_person_character (Utilities|Casting|CastToBP_ThirdPersonCharacter _returnvalue))
  (if (== OtherActor (Game|GetPlayerCharacter 0))
    (Variables|/Game/ThirdPerson/Blueprints/BP_ThirdPersonCharacter.BP_ThirdPersonCharacter_C|SetIsCanInteract? _asbp_third_person_character false)
    (Variables|/Game/ThirdPerson/Blueprints/BP_ThirdPersonCharacter.BP_ThirdPersonCharacter_C|SetCurrentInteractSystem _asbp_third_person_character 0)
    (Widget|RemovefromParent (Variables|Default|GetInteractWidget))))

(event EventBeginPlay
  (|CallParentFunction) ; This node is disabled and will not be called.\nDrag off pins to build functionality.
)

(event Collision|EventActorBeginOverlap
  (params (OtherActor :type Actor%20Object%20Reference))
  (|CallParentFunction OtherActor) ; This node is disabled and will not be called.\nDrag off pins to build functionality.
)

(event EventTick
  (params (DeltaSeconds :type Float%20%28single-precision%29))
  (|CallParentFunction DeltaSeconds) ; This node is disabled and will not be called.\nDrag off pins to build functionality.
)

(fn ConstructionScript
  (|CallParentFunction))

(fn Activation
  (for _array_element (Variables|Default|GetSystemsToActivate)
    (Utilities|IsValid _array_element
      (:Is%20Valid
        (CallFunction|Activation _array_element))))
  (return))