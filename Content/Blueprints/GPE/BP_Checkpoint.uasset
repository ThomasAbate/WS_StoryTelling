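; Checkpoint actor that registers itself as the last checkpoint when the third-person character enters its trigger.
; Each qualifying overlap writes a self reference to LastCheckpoint on the third-person game mode.
; A DoOnce then limits the activation feedback to the first time: a camera shutter sound and Niagara fire spawned at two arrow components.
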(event OnComponentBeginOverlap(Trigger)
  (params (OverlappedComponent :type Primitive%20Component%20Object%20Reference) (OtherActor :type Actor%20Object%20Reference) (OtherComp :type Primitive%20Component%20Object%20Reference) (OtherBodyIndex :type Integer) (bFromSweep :type Boolean) (SweepResult :type Hit%20Result%20Structure%20%28by%20ref%29))
  (Utilities|Casting|CastToBP_ThirdPersonCharacter OtherActor)
  (bind _asbp_third_person_game_mode (Utilities|Casting|CastToBP_ThirdPersonGameMode (Game|GetGameMode)))
  (Variables|/Game/Blueprints/ThirdPerson/Blueprints/BP_ThirdPersonGameMode.BP_ThirdPersonGameMode_C|SetLast%20Checkpoint _asbp_third_person_game_mode self)
  (Utilities|FlowControl|DoOnce false
    (:Completed
      (Audio|PlaySound2D "/Engine/VREditor/Sounds/UI/Camera_Shutter.Camera_Shutter" 1.0 1.0 0.0 0 0)
      (Niagara|SpawnSystematLocation "/Game/GA/VFX/NS_Fire.NS_Fire" (Transformation|GetSocketLocation (Variables|Default|GetArrow) "None"))
      (Niagara|SpawnSystematLocation "/Game/GA/VFX/NS_Fire.NS_Fire" (Transformation|GetSocketLocation (Variables|Default|GetArrow1) "None")))))

(fn ConstructionScript)