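; Moving platform gameplay element, judging by its name the end one, that lifts its mesh when activated.
; The Activation override runs the parent logic, then fires the Anim event.
; Anim uses MoveComponentTo to slide the StaticMesh to a fixed, raised relative height over a short time, with no return movement.
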(event Custom|Anim
  (Components|MoveComponentTo (Variables|Default|GetStaticMesh) (Math|Vector|MakeVector 0.0 0.0 1.8e+03) "0, 0, 0" false false 1.0 false))

(event EventBeginPlay
  (|CallParentFunction) ; This node is disabled and will not be called.\nDrag off pins to build functionality.
)

(event Collision|EventActorBeginOverlap
  (params (OtherActor :type Actor%20Object%20Reference))
  (|CallParentFunction OtherActor) ; This node is disabled and will not be called.\nDrag off pins to build functionality.
)

(event EventTick
  (params (DeltaSeconds :type Float%20%28single-precision%29))
  (|CallParentFunction DeltaSeconds) ; This node is disabled and will not be called.\nDrag off pins to build functionality.
)

(fn ConstructionScript
  (|CallParentFunction))

(fn Activation
  (|CallParentFunction)
  (CallFunction|Anim))