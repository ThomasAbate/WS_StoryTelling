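; Pressure plate Blueprint for a plate-pattern puzzle, giving visual feedback and reporting to a PlatesChecker.
; Activation swaps the mesh to a hue-shift material, while Desactivation restores the basic material and clears the checker's wrong-plate flag.
; Both then ask the checker to re-evaluate success, and both do nothing once the pattern is confirmed.
; The event graph is inactive, so nothing in this Blueprint itself triggers these functions.
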(event EventBeginPlay
  (|CallParentFunction) ; This node is disabled and will not be called.\nDrag off pins to build functionality.
)

(event Collision|EventActorBeginOverlap
  (params (OtherActor :type Actor%20Object%20Reference))
  (|CallParentFunction OtherActor) ; This node is disabled and will not be called.\nDrag off pins to build functionality.
)

(fn ConstructionScript
  (|CallParentFunction))

(fn Activation
  (if (not (Variables|/Game/Blueprints/Level_Systems/System_L_4/BP_PressurePlatePatternChecker.BP_PressurePlatePatternChecker_C|GetPatternIsConfirmed (Variables|Default|GetPlates%20Checker)))
    (Rendering|Material|SetMaterial (Variables|Default|GetPressurePlateMesh) 0 "/Engine/Functions/Engine_MaterialFunctions02/ExampleContent/HueShift_Inst.HueShift_Inst")
    (Default|CheckSuccess (Variables|Default|GetPlates%20Checker))))

(fn Desactivation
  (bind _plates_checker (Variables|Default|GetPlates%20Checker))
  (if (not (Variables|/Game/Blueprints/Level_Systems/System_L_4/BP_PressurePlatePatternChecker.BP_PressurePlatePatternChecker_C|GetPatternIsConfirmed (Variables|Default|GetPlates%20Checker)))
    (Rendering|Material|SetMaterial (Variables|Default|GetPressurePlateMesh) 0 "/Engine/BasicShapes/BasicShapeMaterial.BasicShapeMaterial")
    (Variables|/Game/Blueprints/Level_Systems/System_L_4/BP_PressurePlatePatternChecker.BP_PressurePlatePatternChecker_C|SetIs%20Wrong%20Plate%20Activated _plates_checker false)
    (Default|CheckSuccess _plates_checker)))