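; Tutorial pressure plate whose activation raises two stair actors in a short camera cutscene.
; BeginPlay caches both stair locations, and Activation calls StairUp, which disables player input and blends the view to a designated target.
; The StairAnimation timeline lerps both stairs upward along Z from their cached positions, then blends the view back to the player and restores input.
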(event Custom|Stair%20Up
  (bind _returnvalue (Game|GetPlayerController 0))
  (bind _returnvalue_2 (Game|GetPlayerCharacter 0))
  (bind _returnvalue_3 (Game|GetPlayerController 0))
  (bind _first_stair_location (Variables|Default|GetFirst%20Stair%20Location))
  (bind _second_stair_location (Variables|Default|GetSecond%20Stair%20Location))
  (Input|DisableInput (Game|GetPlayerCharacter 0) _returnvalue)
  (Game|Player|SetViewTargetwithBlend _returnvalue (Variables|Default|GetNew%20View%20Target) 0.2 "VTBlend_PreBlended" 0.2 false)
  (bind _alpha (Timeline|Stair%20Animation Play)
    (:Update
      (Transformation|SetActorLocation (Variables|Default|GetFirst%20Stair) (Math|Vector|Lerp(Vector) _first_stair_location (+ _first_stair_location "0.000000,0.000000,500.000000") _alpha) false false)
      (Transformation|SetActorLocation (Variables|Default|GetSecond%20Stair) (Math|Vector|Lerp(Vector) _second_stair_location (+ _second_stair_location "0.000000,0.000000,500.000000") _alpha) false false))
    (:Finished
      (Game|Player|SetViewTargetwithBlend _returnvalue_3 _returnvalue_2 0.2 "VTBlend_PreBlended" 0.2 false)
      (Input|EnableInput _returnvalue_2 _returnvalue_3))))

(event EventBeginPlay
  (Variables|Default|SetFirst%20Stair%20Location (Transformation|GetActorLocation (Variables|Default|GetFirst%20Stair)))
  (Variables|Default|SetSecond%20Stair%20Location (Transformation|GetActorLocation (Variables|Default|GetSecond%20Stair))))

(fn ConstructionScript
  (|CallParentFunction))

(fn Activation
  (CallFunction|StairUp))