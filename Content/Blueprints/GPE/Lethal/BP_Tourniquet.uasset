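; BP_Tourniquet is a lethal-category hazard that rotates a cube and damages the third-person character on contact.
; From BeginPlay, latent MoveComponentTo calls alternate the cube's yaw target between +90 and -90 degrees, with the Loop and Loop2 events calling each other endlessly.
; The cube's begin-overlap casts the other actor to BP_ThirdPersonCharacter and applies one point of damage.
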(event OnComponentBeginOverlap(Cube)
  (params (OverlappedComponent :type Primitive%20Component%20Object%20Reference) (OtherActor :type Actor%20Object%20Reference) (OtherComp :type Primitive%20Component%20Object%20Reference) (OtherBodyIndex :type Integer) (bFromSweep :type Boolean) (SweepResult :type Hit%20Result%20Structure%20%28by%20ref%29))
  (bind _asbp_third_person_character (Utilities|Casting|CastToBP_ThirdPersonCharacter OtherActor))
  (Game|Damage|ApplyDamage _asbp_third_person_character 1.0 0 0))

(event Custom|Loop
  (Components|MoveComponentTo (Variables|Default|GetCube) "0, 0, 0" "0.000000,-90.000000,0.000000" false false 1.0 false)
  (CallFunction|Loop2))

(event Custom|Loop2
  (Components|MoveComponentTo (Variables|Default|GetCube) "0, 0, 0" "0.000000,90.000000,0.000000" false false 1.0 false)
  (CallFunction|Loop))

(event EventBeginPlay
  (Components|MoveComponentTo (Variables|Default|GetCube) "0, 0, 0" "0.000000,90.000000,0.000000" false false 1.0 false)
  (CallFunction|Loop))

(event Collision|EventActorBeginOverlap
  (params (OtherActor :type Actor%20Object%20Reference)))

(event EventTick
  (params (DeltaSeconds :type Float%20%28single-precision%29)))

(fn ConstructionScript)