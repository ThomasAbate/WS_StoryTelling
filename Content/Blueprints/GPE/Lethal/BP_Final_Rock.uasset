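; Final rock hazard that starts rolling at BeginPlay with sound, camera shake and rumble, locking player input for two seconds.
; A Timeline lerps it to FinalPoint while spinning its sphere.
; Overlapping the player while CanKill is set applies damage and destroys the rock and its BP_Camera_Final_Rock.
; On arrival, End Event clears CanKill, plays impact feedback, blends the view back to the player and enables Box collision.
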(event OnComponentBeginOverlap(Sphere1)
  (params (OverlappedComponent :type Primitive%20Component%20Object%20Reference) (OtherActor :type Actor%20Object%20Reference) (OtherComp :type Primitive%20Component%20Object%20Reference) (OtherBodyIndex :type Integer) (bFromSweep :type Boolean) (SweepResult :type Hit%20Result%20Structure%20%28by%20ref%29))
  ;[0.02083 0.02083 0.02083] Kill the player
  (bind _asbp_third_person_character (Utilities|Casting|CastToBP_ThirdPersonCharacter OtherActor))
  (if (Variables|Default|GetCan%20Kill)
    (Game|Damage|ApplyDamage _asbp_third_person_character 1.0 0 0)
    (Game|Feedback|ClientStopForceFeedback (Game|GetPlayerController 0) "/Game/Blueprints/Feedbacks/Dynamique_FeedBack/FFE_FinalRock.FFE_FinalRock" "None")
    (Actor|DestroyActor)
    (Actor|DestroyActor (Variables|Default|GetCamera))
    (Variables|Default|SetCan%20Kill true)
    (Variables|/Game/Blueprints/Level_Systems/System_L_Rock/BP_Camera_Final_Rock.BP_Camera_Final_Rock_C|SetOne (Variables|Default|GetCamera) true)))

(event Custom|Rock%20Start%20Event
  (bind _returnvalue (Game|GetPlayerController 0))
  (bind _returnvalue_2 (Game|GetPlayerCharacter 0))
  ;[0.02083 0.02083 0.02083] Run Final Rock
  (Audio|PlaySoundatLocation 0 (Transformation|GetActorLocation) "0, 0, 0" 1.0 1.0 0.0 0 0 0 0 :!pinned true) ; Add Sound
  (Class|LegacyCameraShake|StartLegacyCameraShake (Game|GetPlayerCameraManager 0) "/Game/Blueprints/Feedbacks/Camera_Shake/BP_CameraShake_Low.BP_CameraShake_Low_C" 1.0 "CameraLocal" "0, 0, 0")
  (Input|DisableInput _returnvalue_2 _returnvalue)
  (Utilities|FlowControl|Sequence
    (:then_0
      (Game|Feedback|ClientPlayForceFeedback (Game|GetPlayerController 0) "/Game/Blueprints/Feedbacks/Dynamique_FeedBack/FFE_FinalRock.FFE_FinalRock" "None" false false false)
      (bind _newtrack_0 (Timeline|Timeline Play)
        (:Update
          (Transformation|SetRelativeRotation (Variables|Default|GetSphere) (Math|Rotator|Lerp(Rotator) (Variables|Default|GetRoation%20Final%20Rock) "0.000000,0.000000,3600.000000" _newtrack_0) false false)
          (Transformation|SetActorLocation (Math|Vector|Lerp(Vector) (Variables|Default|GetGet%20Default%20Actor%20Location) (Transformation|GetActorLocation (Variables|Default|GetFinal%20Point)) _newtrack_0) false false))
        (:Finished
          (|EndEvent))))
    (:then_1
      (Utilities|FlowControl|Delay 2.0)
      (Input|EnableInput _returnvalue_2 _returnvalue))))

(event EventBeginPlay
  ;[0.02083 0.02083 0.02083] SetUp
  (Collision|SetCollisionEnabled (Variables|Default|GetBox) "NoCollision")
  (bind _returnvalue (Actor|GetActorOfClass "/Game/Blueprints/Level_Systems/System_L_Rock/BP_Camera_Final_Rock.BP_Camera_Final_Rock_C"))
  (Variables|Default|SetCamera _returnvalue)
  (Variables|Default|SetGet%20Default%20Actor%20Location (Transformation|GetActorLocation))
  (Variables|Default|SetRoation%20Final%20Rock (Variables|/Script/Engine.SceneComponent|GetRelativeRotation (Variables|Default|GetSphere)))
  (CallFunction|RockStartEvent))

(fn ConstructionScript)