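; BP_Borne is a rotating pedestal puzzle piece that cycles through four positions from a configurable starting position.
; Activation and Desactivation behave identically, ignoring calls mid-turn, advancing the position with wraparound, then asking the level's BP_BorneChecker to check success before rotation begins.
; RotatingMovement smoothly yaws the Pierre2 component a quarter turn, playing a turning sound during the move and an end sound afterwards.
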(event Custom|RotatingMovement
  (bind _pierre_2 (Variables|Default|GetPierre_2))
  (bind _audiocomponent (Variables|Default|GetAudioComponent))
  (bind _audiocomponent_2 (Variables|Default|GetAudioComponent))
  (Audio|Components|Audio|SetSound _audiocomponent_2 "/Game/Sound/SFX/Bornes/Tourner_Piedestaux.Tourner_Piedestaux")
  (Audio|Components|Audio|Play _audiocomponent_2 0.0)
  (Variables|Default|SetisTurning true)
  (Components|MoveComponentTo _pierre_2 "0, 0, 0" (Math|Rotator|MakeRotator 0.0 0.0 (+ (.yaw (Variables|/Script/Engine.SceneComponent|GetRelativeRotation _pierre_2)) 9e+01)) false false 0.6 false)
  (Audio|Components|Audio|Stop _audiocomponent)
  (Variables|Default|SetisTurning false)
  (Audio|Components|Audio|SetSound _audiocomponent "/Game/Sound/SFX/Bornes/Tourner_Piedestaux_END.Tourner_Piedestaux_END")
  (Audio|Components|Audio|Play _audiocomponent 0.0))

(event EventBeginPlay
  (|CallParentFunction)
  (Variables|Default|SetcurrentPosition (Variables|Default|GetStartingPosition)))

(event Collision|EventActorBeginOverlap
  (params (OtherActor :type Actor%20Object%20Reference))
  (|CallParentFunction OtherActor) ; This node is disabled and will not be called.\nDrag off pins to build functionality.
)

(event EventTick
  (params (DeltaSeconds :type Float%20%28single-precision%29))
  (|CallParentFunction DeltaSeconds) ; This node is disabled and will not be called.\nDrag off pins to build functionality.
)

(fn ConstructionScript
  (|CallParentFunction))

(fn Activation
  (if (not (Variables|Default|GetisTurning))
    (if (>= (Variables|Default|GetcurrentPosition) 4)
      (Variables|Default|SetcurrentPosition 0))
    (Variables|Default|SetcurrentPosition (+ (Variables|Default|GetcurrentPosition) 1))
    (bind _returnvalue (Actor|GetActorOfClass "/Game/Blueprints/Level_Systems/System_L_3/BP_BorneChecker.BP_BorneChecker_C"))
    (Default|CheckSuccess _returnvalue)
    (CallFunction|RotatingMovement)))

(fn Desactivation
  (if (not (Variables|Default|GetisTurning))
    (if (>= (Variables|Default|GetcurrentPosition) 4)
      (Variables|Default|SetcurrentPosition 0))
    (Variables|Default|SetcurrentPosition (+ (Variables|Default|GetcurrentPosition) 1))
    (bind _returnvalue (Actor|GetActorOfClass "/Game/Blueprints/Level_Systems/System_L_3/BP_BorneChecker.BP_BorneChecker_C"))
    (Default|CheckSuccess _returnvalue)
    (CallFunction|RotatingMovement)))