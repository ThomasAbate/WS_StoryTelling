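; BP_FinalAutel is the final altar, a gameplay element that spawns the idol once five or more idol fragments are held.
; It overrides Activation, CheckValidity and CheckCondition, each reading IdoleFragmentCurrent from BP_ThirdPersonGameMode.
; BPLastAutel starts hidden and CheckValidity reveals it at the threshold, while CheckCondition sets Condition to true.
; Activation then runs the parent logic and spawns BP_Idole at the Arrow component's transform.
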(event EventBeginPlay
  (|CallParentFunction)
  (Rendering|SetVisibility (Variables|Default|GetBP_LastAutel) false false))

(event Collision|EventActorBeginOverlap
  (params (OtherActor :type Actor%20Object%20Reference))
  (|CallParentFunction OtherActor) ; This node is disabled and will not be called.\nDrag off pins to build functionality.
)

(event EventTick
  (params (DeltaSeconds :type Float%20%28single-precision%29))
  (|CallParentFunction DeltaSeconds) ; This node is disabled and will not be called.\nDrag off pins to build functionality.
)

(fn ConstructionScript
  (|CallParentFunction))

(fn Activation
  (if (>= (Variables|/Game/Blueprints/ThirdPerson/Blueprints/BP_ThirdPersonGameMode.BP_ThirdPersonGameMode_C|GetIdoleFragmentCurrent (.AsBP%20Third%20Person%20Game%20Mode (Utilities|Casting|CastToBP_ThirdPersonGameMode (Game|GetGameMode)))) 5)
    (|CallParentFunction)
    (Game|SpawnActorfromClass "/Game/GA/MESHES/PROPS/BP_Idole.BP_Idole_C" (Transformation|GetSocketTransform (Variables|Default|GetArrow) "None" "RTS_World") "Undefined" "MultiplyWithRoot" 0 0)))

(fn CheckValidity
  (if (>= (Variables|/Game/Blueprints/ThirdPerson/Blueprints/BP_ThirdPersonGameMode.BP_ThirdPersonGameMode_C|GetIdoleFragmentCurrent (.AsBP%20Third%20Person%20Game%20Mode (Utilities|Casting|CastToBP_ThirdPersonGameMode (Game|GetGameMode)))) 5)
    (Rendering|SetVisibility (Variables|Default|GetBP_LastAutel) true false)))

(fn CheckCondition
  (if (>= (Variables|/Game/Blueprints/ThirdPerson/Blueprints/BP_ThirdPersonGameMode.BP_ThirdPersonGameMode_C|GetIdoleFragmentCurrent (.AsBP%20Third%20Person%20Game%20Mode (Utilities|Casting|CastToBP_ThirdPersonGameMode (Game|GetGameMode)))) 5)
    (Variables|Default|SetCondition true)))