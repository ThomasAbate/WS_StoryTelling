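; BP_FinalDoor is a two-panel sliding door actor with separate DoorOpening and DoorClosing events.
; Each event plays its own timeline, whose DoorCurve lerps the left and right panels' relative locations between hardcoded closed and open positions.
; Opening also pulses light controller force feedback on player 0 every update, while closing prints a leftover debug "Hello" string.
; Nothing in this Blueprint calls either event.
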(event EventBeginPlay
  (|CallParentFunction) ; This node is disabled and will not be called.\nDrag off pins to build functionality.
)

(event Collision|EventActorBeginOverlap
  (params (OtherActor :type Actor%20Object%20Reference))
  (|CallParentFunction OtherActor) ; This node is disabled and will not be called.\nDrag off pins to build functionality.
)

(event EventTick
  (params (DeltaSeconds :type Float%20%28single-precision%29))
  (|CallParentFunction DeltaSeconds) ; This node is disabled and will not be called.\nDrag off pins to build functionality.
)

(event EventDoorOpening
  (bind _doorcurve (Timeline|Timeline_0 Play)
    (:Update
      (Transformation|SetRelativeLocation (Variables|Default|GetDoorLeft) (Math|Vector|Lerp(Vector) "-360.000000,0.000000,0.000000" "-720.000000,0.000000,0.000000" _doorcurve) false false)
      (Transformation|SetRelativeLocation (Variables|Default|GetDoorRight) (Math|Vector|Lerp(Vector) "0.000000,3.500000,14.000000" "360.000000,3.500000,14.000000" _doorcurve) false false)
      (Game|Feedback|PlayDynamicForceFeedback (Game|GetPlayerController 0) 0.1 0.2 true true true true))))

(event EventDoorClosing
  (bind _doorcurve (Timeline|Timeline_1 Play)
    (:Update
      (Transformation|SetRelativeLocation (Variables|Default|GetDoorLeft) (Math|Vector|Lerp(Vector) "-720.000000,0.000000,0.000000" "-360.000000,0.000000,0.000000" _doorcurve) false false)
      (Transformation|SetRelativeLocation (Variables|Default|GetDoorRight) (Math|Vector|Lerp(Vector) "360.000000,3.500000,14.000000" "0.000000,3.500000,14.000000" _doorcurve) false false)
      (Development|PrintString "Hello"))))

(fn ConstructionScript
  (|CallParentFunction))