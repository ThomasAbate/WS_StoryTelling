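; Pressure plate Blueprint that switches a set of linked systems on and off.
; The Activation and Desactivation functions relay the matching call to every entry in the SystemToActivates array.
; Separate Activated and Deactivated events handle the visual feedback, using MoveComponentTo to sink and raise the CrystalPlaque1 component.
; No overlap detection or calls to these functions and events appear in these graphs.
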(event Custom|Activated
  (Components|MoveComponentTo (Variables|Default|GetCrystal_Plaque1) "130.000000,15.000000,-10.000000" "0, 0, 0" false false 0.2 false))

(event Custom|Deactivated
  (Components|MoveComponentTo (Variables|Default|GetCrystal_Plaque1) "130.000000,15.000000,0.000000" "0, 0, 0" false false 0.2 false))

(event EventBeginPlay
  (|CallParentFunction) ; This node is disabled and will not be called.\nDrag off pins to build functionality.
)

(event Collision|EventActorBeginOverlap
  (params (OtherActor :type Actor%20Object%20Reference))
  (|CallParentFunction OtherActor) ; This node is disabled and will not be called.\nDrag off pins to build functionality.
)

(event EventTick
  (params (DeltaSeconds :type Float%20%28single-precision%29))
  (|CallParentFunction DeltaSeconds) ; This node is disabled and will not be called.\nDrag off pins to build functionality.
)

(fn ConstructionScript
  (|CallParentFunction))

(fn Activation
  (for _array_element (Variables|Default|GetSystemToActivates)
    (CallFunction|Activation _array_element)))

(fn Desactivation
  (for _array_element (Variables|Default|GetSystemToActivates)
    (CallFunction|Desactivation _array_element)))