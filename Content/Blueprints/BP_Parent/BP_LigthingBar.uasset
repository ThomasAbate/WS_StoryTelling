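; BP_LigthingBar is a parent Blueprint for a bar mesh that switches between a basic and an activated look.
; On BeginPlay it applies BasicMaterial to slot 0 of its StaticMesh.
; The Activation and Desactivation functions swap that slot to ActivatedMaterial or back to BasicMaterial, with no internal trigger, so the calls must come from outside.
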(event EventBeginPlay
  (Rendering|Material|SetMaterial (Variables|Default|GetStaticMesh) 0 (Variables|Default|GetBasicMaterial)))

(event Collision|EventActorBeginOverlap
  (params (OtherActor :type Actor%20Object%20Reference))
  (|CallParentFunction OtherActor) ; This node is disabled and will not be called.\nDrag off pins to build functionality.
)

(event EventTick
  (params (DeltaSeconds :type Float%20%28single-precision%29))
  (|CallParentFunction DeltaSeconds) ; This node is disabled and will not be called.\nDrag off pins to build functionality.
)

(fn ConstructionScript
  (|CallParentFunction))

(fn Activation
  (Rendering|Material|SetMaterial (Variables|Default|GetStaticMesh) 0 (Variables|Default|GetActivatedMaterial)))

(fn Desactivation
  (Rendering|Material|SetMaterial (Variables|Default|GetStaticMesh) 0 (Variables|Default|GetBasicMaterial)))