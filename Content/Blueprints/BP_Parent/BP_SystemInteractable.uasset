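; Base interactable system Blueprint that lets the player interact inside a box trigger and relays activation to other systems.
; Player overlap registers it as the character's current interactable and shows a prompt widget, unless already used once-only or failing the optional CheckCondition, an empty hook here.
; Leaving disables interaction and removes the widget, but still leaves the character's reference pointing here.
; Activation and Desactivation forward to every valid entry in SystemsToActivate.
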(event OnComponentBeginOverlap(Box)
  (params (OverlappedComponent :type Primitive%20Component%20Object%20Reference) (OtherActor :type Actor%20Object%20Reference) (OtherComp :type Primitive%20Component%20Object%20Reference) (OtherBodyIndex :type Integer) (bFromSweep :type Boolean) (SweepResult :type Hit%20Result%20Structure%20%28by%20ref%29))
  (bind _returnvalue (Game|GetPlayerCharacter 0))
  (bind _asbp_third_person_character (Utilities|Casting|CastToBP_ThirdPersonCharacter _returnvalue))
  (if (not (and (Variables|Default|GetInteractableOnce) (Variables|Default|GetisInteracted)))
    (if (== OtherActor _returnvalue)
      (if (Variables|Default|GetHaveCondition)
        (CallFunction|CheckCondition)
        (if (Variables|Default|GetCondition)
          (Variables|/Game/Blueprints/ThirdPerson/Blueprints/BP_ThirdPersonCharacter.BP_ThirdPersonCharacter_C|SetIsCanInteract? _asbp_third_person_character true :!label _label)
          (Variables|/Game/Blueprints/ThirdPerson/Blueprints/BP_ThirdPersonCharacter.BP_ThirdPersonCharacter_C|SetCurrentInteractSystem _asbp_third_person_character self)
          (bind _returnvalue_2 (UserInterface|CreateWidget (Variables|Default|GetWidget) (Game|GetPlayerController 0)))
          (bind _output_get (Variables|Default|SetInteractWidget _returnvalue_2))
          (UserInterface|Viewport|AddtoViewport _output_get 0))
        (else
          (goto _label))))))

(event OnComponentEndOverlap(Box)
  (params (OverlappedComponent :type Primitive%20Component%20Object%20Reference) (OtherActor :type Actor%20Object%20Reference) (OtherComp :type Primitive%20Component%20Object%20Reference) (OtherBodyIndex :type Integer))
  (bind _returnvalue (Game|GetPlayerCharacter 0))
  (bind _interactwidget (Variables|Default|GetInteractWidget))
  (bind _asbp_third_person_character (Utilities|Casting|CastToBP_ThirdPersonCharacter _returnvalue))
  (if (== OtherActor (Game|GetPlayerCharacter 0))
    (Variables|/Game/Blueprints/ThirdPerson/Blueprints/BP_ThirdPersonCharacter.BP_ThirdPersonCharacter_C|SetIsCanInteract? _asbp_third_person_character false)
    (Variables|/Game/Blueprints/ThirdPerson/Blueprints/BP_ThirdPersonCharacter.BP_ThirdPersonCharacter_C|SetCurrentInteractSystem _asbp_third_person_character self)
    (Utilities|IsValid _interactwidget
      (:Is%20Valid
        (Widget|RemovefromParent _interactwidget)))))

(event EventBeginPlay
  (|CallParentFunction) ; This node is disabled and will not be called.\nDrag off pins to build functionality.
)

(event Collision|EventActorBeginOverlap
  (params (OtherActor :type Actor%20Object%20Reference))
  (|CallParentFunction OtherActor) ; This node is disabled and will not be called.\nDrag off pins to build functionality.
)

(event EventTick
  (params (DeltaSeconds :type Float%20%28single-precision%29))
  (|CallParentFunction DeltaSeconds) ; This node is disabled and will not be called.\nDrag off pins to build functionality.
)

(fn ConstructionScript
  (|CallParentFunction))

(fn Activation
  (for _array_element (Variables|Default|GetSystemsToActivate)
    (Utilities|IsValid _array_element
      (:Is%20Valid
        (CallFunction|Activation _array_element))))
  (return))

(fn Desactivation
  (for _array_element (Variables|Default|GetSystemsToActivate)
    (Utilities|IsValid _array_element
      (:Is%20Valid
        (CallFunction|Desactivation _array_element))))
  (return))

(fn CheckCondition)