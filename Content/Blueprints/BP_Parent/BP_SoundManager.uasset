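; BP_SoundManager is a Blueprint that shifts the game's ambience to a darker track through a transition sound.
; Activation reads the audio components on BP_ThirdPersonGameMode, plays TransitionAmbience and stops MainAmbience.
; PlaySoundWithAutoTransition binds the transition's OnAudioFinished to PlayNewSound, which starts AmbienceDarker, with debug prints along the way.
; PassToDarkAmbience is an empty stub.
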(event Custom|PlaySoundWithAutoTransition
  (params (Original%20Sound :type Audio%20Component%20Object%20Reference) (New%20Sound :type Audio%20Component%20Object%20Reference))
  (EventDispatchers|BindEventtoOnAudioFinished Original%20Sound (delegate Custom|PlayNewSound))
  (Development|PrintString "Dark ambience ready to play"))

(event Custom|PlayNewSound
  (Audio|Components|Audio|Play (stale Custom|PlaySoundWithAutoTransition New%20Sound) 0.0)
  (Development|PrintString "Play dark ambience"))

(event EventBeginPlay
  (|CallParentFunction) ; This node is disabled and will not be called.\nDrag off pins to build functionality.
)

(event Collision|EventActorBeginOverlap
  (params (OtherActor :type Actor%20Object%20Reference))
  (|CallParentFunction OtherActor) ; This node is disabled and will not be called.\nDrag off pins to build functionality.
)

(event EventTick
  (params (DeltaSeconds :type Float%20%28single-precision%29))
  (|CallParentFunction DeltaSeconds) ; This node is disabled and will not be called.\nDrag off pins to build functionality.
)

(fn ConstructionScript
  (|CallParentFunction))

(fn Activation
  (bind _returnvalue (Game|GetGameMode))
  (bind _asbp_third_person_game_mode (Utilities|Casting|CastToBP_ThirdPersonGameMode _returnvalue))
  (bind _transitionambience (Variables|/Game/Blueprints/ThirdPerson/Blueprints/BP_ThirdPersonGameMode.BP_ThirdPersonGameMode_C|GetTransitionAmbience _asbp_third_person_game_mode))
  (Audio|Components|Audio|Play _transitionambience 0.0)
  (Development|PrintString "Transition")
  (Audio|Components|Audio|Stop (Variables|/Game/Blueprints/ThirdPerson/Blueprints/BP_ThirdPersonGameMode.BP_ThirdPersonGameMode_C|GetMainAmbience _asbp_third_person_game_mode))
  (CallFunction|PlaySoundwithAutoTransition _transitionambience (Variables|/Game/Blueprints/ThirdPerson/Blueprints/BP_ThirdPersonGameMode.BP_ThirdPersonGameMode_C|GetAmbienceDarker _asbp_third_person_game_mode)))

(fn PasstoDarkAmbience)